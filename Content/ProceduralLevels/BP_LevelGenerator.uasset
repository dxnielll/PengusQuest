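; Procedural level generator that builds a chain of rooms on BeginPlay, from a starting room through three sections to an ending room.
; Each room spawns at the previous ExitPoint's location, with section rooms picked at random from arrays in each section master's class defaults.
; A seeded stream, created once and stored in the save, reproduces the layout.
; Section 2 runs its random pass twice; its start-room event is never called.
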(event `SpawnLastRoom`
  ;[0.901 0.6908 0.006562 0.5] Spawn Ending Room
  (bind _returnvalue (`|SpawnActorFromClass` "/Game/ProceduralLevels/BP_EndingTestRoom.BP_EndingTestRoom_C" (`KismetMathLibrary.MakeTransform` (`SceneComponent.K2_GetComponentLocation` (`self.ExitPoint`))) "AlwaysSpawn" "MultiplyWithRoot" null null))
  (set `self.LatestRoom` _returnvalue)
  (set `self.ExitPoint` (`/Game/ProceduralLevels/BP_Master_Room.ExitPoint` _returnvalue)))

(event `SpawnSection3`
  ;[0 0.02034 1 0.5] Spawn Section 3
  (for _ (range 1 (+ (`self.RoomsPerSection`) 1))
    (bind _returnvalue (`|SpawnActorFromClass` (`KismetArrayLibrary.Array_RandomFromStream` (`self.RoomSection3`) (`self.Stream`)) (`KismetMathLibrary.MakeTransform` (`SceneComponent.K2_GetComponentLocation` (`self.ExitPoint`))) "AlwaysSpawn" "MultiplyWithRoot" null null))
    (bind _asbp_master_room (cast `/Game/ProceduralLevels/BP_Master_Room` _returnvalue :!pure true))
    (set `self.LatestRoom` _asbp_master_room)
    (set `self.ExitPoint` (`/Game/ProceduralLevels/BP_Master_Room.ExitPoint` _asbp_master_room))))

(event `SpawnStartSection3`
  ;[0.007466 0.000328 0.15 0.5] Spawn Start Section 3
  (bind _returnvalue (`|SpawnActorFromClass` "/Game/ProceduralLevels/BP_Section3_Master_TestRoom.BP_Section3_Master_TestRoom_C" (`KismetMathLibrary.MakeTransform` (`SceneComponent.K2_GetComponentLocation` (`self.ExitPoint`))) "AlwaysSpawn" "MultiplyWithRoot" null null))
  (set `self.LatestRoom` _returnvalue)
  (set `self.ExitPoint` (`/Game/ProceduralLevels/BP_Master_Room.ExitPoint` _returnvalue)))

(event `SpawnSection2`
  ;[1 0 0.311 0.5] Spawn Section 2
  (for _ (range 1 (+ (`self.RoomsPerSection`) 1))
    (bind _returnvalue (`|SpawnActorFromClass` (`KismetArrayLibrary.Array_RandomFromStream` (`self.RoomSection2`) (`self.Stream`)) (`KismetMathLibrary.MakeTransform` (`SceneComponent.K2_GetComponentLocation` (`self.ExitPoint`))) "AlwaysSpawn" "MultiplyWithRoot" null null))
    (bind _asbp_master_room (cast `/Game/ProceduralLevels/BP_Master_Room` _returnvalue :!pure true))
    (set `self.LatestRoom` _asbp_master_room)
    (set `self.ExitPoint` (`/Game/ProceduralLevels/BP_Master_Room.ExitPoint` _asbp_master_room))))

(event `SpawnStartSection2`
  ;[0.5729 0 0.2187 0.5] Spawn Start Section 2
  (bind _returnvalue (`|SpawnActorFromClass` "/Game/ProceduralLevels/BP_Section2_Master_TestRoom.BP_Section2_Master_TestRoom_C" (`KismetMathLibrary.MakeTransform` (`SceneComponent.K2_GetComponentLocation` (`self.ExitPoint`))) "AlwaysSpawn" "MultiplyWithRoot" null null))
  (set `self.LatestRoom` _returnvalue)
  (set `self.ExitPoint` (`/Game/ProceduralLevels/BP_Master_Room.ExitPoint` _returnvalue)))

(event `SpawnSection1`
  ;[0.7336 0 0.7552 0.5] Spawn Section 1
  (for _ (range 1 (+ (`self.RoomsPerSection`) 1))
    (bind _returnvalue (`|SpawnActorFromClass` (`KismetArrayLibrary.Array_RandomFromStream` (`self.RoomSection1`) (`self.Stream`)) (`KismetMathLibrary.MakeTransform` (`SceneComponent.K2_GetComponentLocation` (`self.ExitPoint`))) "AlwaysSpawn" "MultiplyWithRoot" null null))
    (bind _asbp_master_room (cast `/Game/ProceduralLevels/BP_Master_Room` _returnvalue :!pure true))
    (set `self.LatestRoom` _asbp_master_room)
    (set `self.ExitPoint` (`/Game/ProceduralLevels/BP_Master_Room.ExitPoint` _asbp_master_room))))

(event `SetSeed`
  (bind _seed (`/Game/Blueprints/BP_SaveData.seed` (`self.Save Ref`)))
  ; Set Seed
  (if (== _seed -1)
    (bind _output_get (set `/Game/Blueprints/BP_SaveData.seed` (`KismetMathLibrary.RandomInteger` 100000) (`self.Save Ref`)))
    (set `self.Seed` _output_get)
    (`KismetMathLibrary.SetRandomStreamSeed` (`self.Stream`) (`self.Seed`))
    (else
      (bind _output_get_2 (set `self.Seed` _seed))
      (`KismetMathLibrary.SetRandomStreamSeed` (`self.Stream`) _output_get_2))))

(event `SpawnStartSection1`
  ;[0.5677 0.007362 0.5462 0.5] Spawn Start Section 1
  (bind _returnvalue (`|SpawnActorFromClass` "/Game/ProceduralLevels/BP_Section1_Master_TestRoom.BP_Section1_Master_TestRoom_C" (`KismetMathLibrary.MakeTransform` (`SceneComponent.K2_GetComponentLocation` (`self.ExitPoint`))) "AlwaysSpawn" "MultiplyWithRoot" null null))
  (set `self.LatestRoom` _returnvalue)
  (set `self.ExitPoint` (`/Game/ProceduralLevels/BP_Master_Room.ExitPoint` _returnvalue)))

(event `StoreRoomSections`
  (set `self.RoomSection1` (defaults `/Game/ProceduralLevels/BP_Section1_Master_TestRoom` "/Game/ProceduralLevels/BP_Section1_Master_TestRoom.BP_Section1_Master_TestRoom_C"))
  (set `self.RoomSection2` (defaults `/Game/ProceduralLevels/BP_Section2_Master_TestRoom` "/Game/ProceduralLevels/BP_Section2_Master_TestRoom.BP_Section2_Master_TestRoom_C"))
  (set `self.RoomSection3` (defaults `/Game/ProceduralLevels/BP_Section3_Master_TestRoom` "/Game/ProceduralLevels/BP_Section3_Master_TestRoom.BP_Section3_Master_TestRoom_C")))

(event `SpawnStartRoom`
  ;[0.15 0 0.01889 0.5] Spawn Starting Room
  (bind _returnvalue (`|SpawnActorFromClass` "/Game/ProceduralLevels/BP_StartingTestRoom.BP_StartingTestRoom_C" (`SceneComponent.K2_GetComponentToWorld` (`self.DefaultSceneRoot`)) "AlwaysSpawn" "MultiplyWithRoot" null null))
  (set `self.ExitPoint` (`/Game/ProceduralLevels/BP_Master_Room.ExitPoint` _returnvalue)))

(event `self.ReceiveBeginPlay`
  (bind _asbp_game_instance (cast `/Game/Blueprints/BP_GameInstance` (`GameplayStatics.GetGameInstance`) :!pure true))
  (set `self.Save Ref` (`/Game/Blueprints/BP_GameInstance.SaveRef` _asbp_game_instance))
  (`self.StoreRoomSections`)
  (`self.SetSeed`)
  (`self.SpawnStartRoom`)
  (`self.SpawnStartSection1`)
  (`self.SpawnSection1`)
  (`self.SpawnSection2`)
  (`self.SpawnSection2`)
  (`self.SpawnStartSection3`)
  (`self.SpawnSection3`)
  (`self.SpawnLastRoom`)
  (`/Game/Blueprints/BP_GameInstance.SaveGame` _asbp_game_instance (`/Game/Blueprints/BP_GameInstance.CurrentSlotName` _asbp_game_instance)))

(fn `UserConstructionScript`)