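; BP_EndingTestRoom is an ending room for the procedural levels that closes out the player's run.
; When the player character overlaps the Ending volume before having finished, it destroys the Fallingplt component, waits briefly, then calls FinishRun on the character.
; A ShowHideWidgets helper collapses one list of widgets and shows another, but the shown graphs never call it.
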(event `self.Ending.OnComponentBeginOverlap`
  (params (OverlappedComponent :type "PrimitiveComponent Object Reference") (OtherActor :type "Actor Object Reference") (OtherComp :type "PrimitiveComponent Object Reference") (OtherBodyIndex :type Integer) (bFromSweep :type Boolean) (SweepResult :type "HitResult Structure (by ref)"))
  (bind _playercharacter (`self.PlayerCharacter`))
  (bind _fallingplt (`self.fallingplt`))
  (if (and (== OtherActor _playercharacter) (not (`/Game/ThirdPerson/Blueprints/BP_ThirdPersonCharacter.hasFinished` _playercharacter)))
    (`/Engine/EditorBlueprintResources/StandardMacros.IsValid` _fallingplt
      (:`Is Valid`
        (`ActorComponent.K2_DestroyComponent` _fallingplt))
      (:`Is Not Valid`
        _))
    (`KismetSystemLibrary.Delay` 3.0)
    (`/Game/ThirdPerson/Blueprints/BP_ThirdPersonCharacter.FinishRun` _playercharacter)))

(fn `ShowHideWidgets`
  (params (widgetsToHide :type "Array of Widget Object Reference") (widgetsToShow :type "Array of Widget Object Reference"))
  (for _array_element widgetsToHide
    (`Widget.SetVisibility` _array_element "Collapsed"))
  (for _array_element_2 widgetsToShow
    (`Widget.SetVisibility` _array_element_2 "SelfHitTestInvisible")))

(fn `UserConstructionScript`
  (`parent.UserConstructionScript`))