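; Level generator actor that builds a level by chaining room Blueprints, spawning each at the previous room's ExitPoint.
; GenerateLevels currently spawns a fixed test sequence: start room, three sections each led by a master room, then ending room.
; A disconnected original path seeds a random stream and picks rooms from per-section arrays, which BeginPlay loads from master-room class defaults.
; That path's removal step re-rolls the stream, so it may remove a different room than spawned.
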(event `SpawnStartRoom`
  ; RoomGeneration
  (bind _returnvalue (`|SpawnActorFromClass` "/Game/ProceduralLevels/BP_StartingTestRoom.BP_StartingTestRoom_C" (`SceneComponent.K2_GetComponentToWorld` (`self.DefaultSceneRoot`)) "AlwaysSpawn" "MultiplyWithRoot" null null))
  (set `self.ExitPoint` (`/Game/ProceduralLevels/BP_Master_Room.ExitPoint` _returnvalue)))

(event `SetSeed`
  (params (Seed :type Integer) (SaveRef :type "/Game/Blueprints/BP_SaveData Object Reference"))
  ; Set Seed
  (if (== Seed -1)
    (bind _output_get (set `/Game/Blueprints/BP_SaveData.seed` (`KismetMathLibrary.RandomInteger` 99999) SaveRef))
    (set `self.Seed` _output_get)
    (`KismetMathLibrary.SetRandomStreamSeed` (`self.Stream`) (`self.Seed`))
    (else
      (bind _output_get_2 (set `self.Seed` Seed))
      (`KismetMathLibrary.SetRandomStreamSeed` (`self.Stream`) _output_get_2))))

(event `SpawnStartSection1`
  ; RoomGeneration
  (`self.SpawnSetRoom` "/Game/ProceduralLevels/BP_Section1_Master_TestRoom.BP_Section1_Master_TestRoom_C"))

(event `SpawnStartSection2`
  ; RoomGeneration
  (`self.SpawnSetRoom` "/Game/ProceduralLevels/BP_Section2_Master_TestRoom.BP_Section2_Master_TestRoom_C"))

(event `SpawnStartSection3`
  ; RoomGeneration
  (`self.SpawnSetRoom` "/Game/ProceduralLevels/BP_Section3_Master_TestRoom.BP_Section3_Master_TestRoom_C"))

(event `SpawnLastRoom`
  ; RoomGeneration
  (`self.SpawnSetRoom` "/Game/ProceduralLevels/BP_EndingTestRoom.BP_EndingTestRoom_C"))

(event `SpawnSection1`
  ; RoomGeneration
  (`self.SpawnRandomRoomFromArray` (`self.RoomSection1`)))

(event `SpawnSection2`
  ; RoomGeneration
  (`self.SpawnRandomRoomFromArray` (`self.RoomSection2`)))

(event `SpawnSection3`
  ; RoomGeneration
  (`self.SpawnRandomRoomFromArray` (`self.RoomSection3`)))

(event `self.ReceiveBeginPlay`
  (`self.StoreRoomSections`))

(fn `GenerateLevels`
  (params (Seed :type Integer) (SaveRef :type "/Game/Blueprints/BP_SaveData Object Reference"))
  (`self.SpawnSetRoom` "/Game/ProceduralLevels/BP_StartingTestRoom.BP_StartingTestRoom_C")
  (`self.SpawnSetRoom` "/Game/ProceduralLevels/BP_Section1_Master_TestRoom.BP_Section1_Master_TestRoom_C")
  (`self.SpawnSetRoom` "/Game/ProceduralLevels/Section_1/BP_Section1_TestRoom_1.BP_Section1_TestRoom_1_C")
  (`self.SpawnSetRoom` "/Game/ProceduralLevels/Section_1/BP_Section1_TestRoom_2.BP_Section1_TestRoom_2_C")
  (`self.SpawnSetRoom` "/Game/ProceduralLevels/Section_1/BP_Section1_TestRoom_3.BP_Section1_TestRoom_3_C")
  (`self.SpawnSetRoom` "/Game/ProceduralLevels/Section_1/BP_Section1_TestRoom_4.BP_Section1_TestRoom_4_C")
  (`self.SpawnSetRoom` "/Game/ProceduralLevels/Section_1/BP_Section1_TestRoom_5.BP_Section1_TestRoom_5_C")
  (`self.SpawnSetRoom` "/Game/ProceduralLevels/BP_Section2_Master_TestRoom.BP_Section2_Master_TestRoom_C")
  (`self.SpawnSetRoom` "/Game/ProceduralLevels/Section_2/BP_Section2_TestRoom_1.BP_Section2_TestRoom_1_C")
  (`self.SpawnSetRoom` "/Game/ProceduralLevels/Section_2/BP_Section2_TestRoom_2.BP_Section2_TestRoom_2_C")
  (`self.SpawnSetRoom` "/Game/ProceduralLevels/Section_2/BP_Section2_TestRoom_3.BP_Section2_TestRoom_3_C")
  (`self.SpawnSetRoom` "/Game/ProceduralLevels/Section_2/BP_Section2_TestRoom_4.BP_Section2_TestRoom_4_C")
  (`self.SpawnSetRoom` "/Game/ProceduralLevels/Section_2/BP_Section2_TestRoom_5.BP_Section2_TestRoom_5_C")
  (`self.SpawnSetRoom` "/Game/ProceduralLevels/BP_Section3_Master_TestRoom.BP_Section3_Master_TestRoom_C")
  (`self.SpawnSetRoom` "/Game/ProceduralLevels/Section_3/BP_Section3_TestRoom_1.BP_Section3_TestRoom_1_C")
  (`self.SpawnSetRoom` "/Game/ProceduralLevels/Section_3/BP_Section3_TestRoom_2.BP_Section3_TestRoom_2_C")
  (`self.SpawnSetRoom` "/Game/ProceduralLevels/Section_3/BP_Section3_TestRoom_3.BP_Section3_TestRoom_3_C")
  (`self.SpawnSetRoom` "/Game/ProceduralLevels/Section_3/BP_Section3_TestRoom_4.BP_Section3_TestRoom_4_C")
  (`self.SpawnSetRoom` "/Game/ProceduralLevels/Section_3/BP_Section3_TestRoom_5.BP_Section3_TestRoom_5_C")
  (`self.SpawnSetRoom` "/Game/ProceduralLevels/BP_EndingTestRoom.BP_EndingTestRoom_C"))

(fn `SpawnRandomRoomFromArray`
  (params (RoomArray :type "Array of Actor Class Reference (by ref)"))
  (bind (_outitem _outindex) (`KismetArrayLibrary.Array_RandomFromStream` RoomArray (`self.Stream`)))
  (for _ (range 1 (+ (`self.RoomsPerSection`) 1))
    (bind _returnvalue (`|SpawnActorFromClass` _outitem (`KismetMathLibrary.MakeTransform` (`SceneComponent.K2_GetComponentLocation` (`self.ExitPoint`))) "AlwaysSpawn" "MultiplyWithRoot" null null))
    (bind _asbp_master_room (cast `/Game/ProceduralLevels/BP_Master_Room` _returnvalue :!pure true))
    (set `self.LatestRoom` _asbp_master_room)
    (set `self.ExitPoint` (`/Game/ProceduralLevels/BP_Master_Room.ExitPoint` _asbp_master_room))
    (`KismetSystemLibrary.PrintString` (`KismetStringLibrary.Concat_StrStr` "spawned room: " (`KismetSystemLibrary.GetDisplayName` _returnvalue)) true true (struct :`G` 0.66 :`B` 1.0 :`A` 1.0) 10.0)
    (`KismetArrayLibrary.Array_Remove` (`local.RoomArray`) _outindex)))

(fn `SpawnSetRoom`
  (params (Room :type "Actor Class Reference"))
  (bind _returnvalue (`|SpawnActorFromClass` Room (`KismetMathLibrary.MakeTransform` (`SceneComponent.K2_GetComponentLocation` (`self.ExitPoint`))) "AlwaysSpawn" "MultiplyWithRoot" null null))
  (bind _asbp_master_room (cast `/Game/ProceduralLevels/BP_Master_Room` _returnvalue :!pure true))
  (set `self.LatestRoom` _asbp_master_room)
  (set `self.ExitPoint` (`/Game/ProceduralLevels/BP_Master_Room.ExitPoint` _asbp_master_room)))

(fn `StoreRoomSections`
  (set `self.RoomSection1` (defaults `/Game/ProceduralLevels/BP_Section1_Master_TestRoom` "/Game/ProceduralLevels/BP_Section1_Master_TestRoom.BP_Section1_Master_TestRoom_C"))
  (set `self.RoomSection2` (defaults `/Game/ProceduralLevels/BP_Section2_Master_TestRoom` "/Game/ProceduralLevels/BP_Section2_Master_TestRoom.BP_Section2_Master_TestRoom_C"))
  (set `self.RoomSection3` (defaults `/Game/ProceduralLevels/BP_Section3_Master_TestRoom` "/Game/ProceduralLevels/BP_Section3_Master_TestRoom.BP_Section3_Master_TestRoom_C")))

(fn `UserConstructionScript`)