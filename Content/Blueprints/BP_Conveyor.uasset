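; Conveyor belt actor that carries overlapping third-person characters along its surface.
; Each tick it offsets characters inside the Box trigger along the Arrow's forward direction by Speed, without sweeping.
; On BeginPlay a dynamic material instance sets the belt texture scroll rate from the same Speed.
; The construction script uses HasHelperCube to show a collidable HelperCube and resize the trigger box to match.
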(event `self.ReceiveBeginPlay`
  (bind _returnvalue (`PrimitiveComponent.CreateDynamicMaterialInstance` (`self.Conveyor`) 0 "/Game/Materials/MM_Conveyor.MM_Conveyor" "None"))
  (`MaterialInstanceDynamic.SetScalarParameterValue` _returnvalue "Speed_Tex_Val" (/ (`self.Speed`) 360.0)))

(event `self.ReceiveTick`
  (params (DeltaSeconds :type "Float (single-precision)"))
  (for _array_element (`PrimitiveComponent.GetOverlappingActors` (`self.Box`) "/Game/ThirdPerson/Blueprints/BP_ThirdPersonCharacter.BP_ThirdPersonCharacter_C")
    (`self.K2_AddActorWorldOffset` _array_element (* (* DeltaSeconds (`self.Speed`)) (`KismetMathLibrary.GetForwardVector` (`SceneComponent.K2_GetComponentRotation` (`self.Arrow`)))) false false)))

(fn `UserConstructionScript`
  (bind _helpercube (`self.HelperCube`))
  (bind _helpercube_2 (`self.HelperCube`))
  (bind _box (`self.Box`))
  (if (`self.HasHelperCube`)
    (`SceneComponent.SetHiddenInGame` _helpercube_2 false false)
    (`PrimitiveComponent.SetCollisionEnabled` _helpercube_2 "QueryAndPhysics")
    (`BoxComponent.SetBoxExtent` _box (49.360486 42.595178 27.328449) true)
    (else
      (`SceneComponent.SetHiddenInGame` _helpercube true false)
      (`PrimitiveComponent.SetCollisionEnabled` _helpercube "NoCollision")
      (`BoxComponent.SetBoxExtent` _box (49.360486 50.284996 27.328449) true))))